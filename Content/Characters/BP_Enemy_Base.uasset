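; Base enemy character Blueprint that provides attack, weapon, movement speed and patrol functions.
; Attack plays a test montage and fires OnAttackEnd whether it completes or is interrupted.
; WieldWeapon spawns a spear, snaps it to a hand socket and flags the weapon as wielded.
; Getters expose fixed attack and defend radii and the patrol route, while SetMovementSpeed maps speed states to walk speed, overriding the BeginPlay default.
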(event `self.ReceiveBeginPlay`
  (set `CharacterMovementComponent.MaxWalkSpeed` 110.0 (`self.CharacterMovement`)))

(event `Attack`
  (`|PlayMontage` (`self.Mesh`) "/Game/Characters/Bosses/SpectralWarden/Animations/Spectral_Warden_TestAttack_Montage2.Spectral_Warden_TestAttack_Montage2"
    (:`OnCompleted`
      _)
    (:`OnInterrupted`
      _))
  (`self.OnAttackEnd`))

(event `WieldWeapon`
  (bind _returnvalue (`|SpawnActorFromClass` "/Game/Weapons/Blueprints/BP_Spear.BP_Spear_C" (`self.GetTransform`) "Undefined" "MultiplyWithRoot" null null))
  (`self.K2_AttachToComponent` _returnvalue (`self.Mesh`) "hand_rSocket_spear" "SnapToTarget" "SnapToTarget" "SnapToTarget" true)
  (set `self.IsWieldingWeapon` true))

(fn `GetIdealRange`
  (returns (AttackRadius :type "Float (double-precision)") (DefendRadius :type "Float (double-precision)"))
  (return 350.0 350.0))

(fn `GetPatrolRoute`
  (returns (PatrolRoute :type "/Game/Characters/Ai/BP_PatrolRoute Object Reference"))
  (return (`self.PatrolRoute`)))

(fn `SetMovementSpeed`
  (params (Speed :type "/Game/Characters/Ai/Enums/E_MovementSpeed Enum" :default "NewEnumerator0"))
  (returns (SpeedValue :type "Float (double-precision)"))
  (bind _output_get (set `CharacterMovementComponent.MaxWalkSpeed` (select `/Game/Characters/Ai/Enums/E_MovementSpeed` Speed :`NewEnumerator1` 100.0 :`NewEnumerator2` 300.0 :`NewEnumerator3` 500.0 :!type "Float (single-precision)") (`self.CharacterMovement`)))
  (return _output_get))

(fn `UserConstructionScript`)