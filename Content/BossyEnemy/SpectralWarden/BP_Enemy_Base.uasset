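; Base Blueprint for the Spectral Warden enemy, providing its walk speed, attack, weapon wielding and patrol route access.
; Attack plays a test attack montage and calls OnAttackEnd whether it completes or is interrupted.
; WieldWeapon spawns a spear, snaps it to the right-hand socket and sets IsWieldingSword, despite the weapon being a spear.
; GetPatrolRoute returns the stored route, while BeginPlay caps movement at a slow walk.
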(event `self.ReceiveBeginPlay`
  (set `CharacterMovementComponent.MaxWalkSpeed` 110.0 (`self.CharacterMovement`)))

(event `Attack`
  (`|PlayMontage` (`self.Mesh`) "/Game/BossyEnemy/SpectralWarden/Animations/Spectral_Warden_TestAttacj_Montage2.Spectral_Warden_TestAttacj_Montage2"
    (:`OnCompleted`
      _)
    (:`OnInterrupted`
      _))
  (`self.OnAttackEnd`))

(event `WieldWeapon`
  (bind _returnvalue (`|SpawnActorFromClass` "/Game/Weapons/BP_Spear.BP_Spear_C" (`self.GetTransform`) "Undefined" "MultiplyWithRoot" null null))
  (`self.K2_AttachToComponent` _returnvalue (`self.Mesh`) "hand_rSocket_spear" "SnapToTarget" "SnapToTarget" "SnapToTarget" true)
  (set `self.IsWieldingSword` true))

(fn `GetPatrolRoute`
  (returns (PatrolRoute :type "/Game/BossyEnemy/SpectralWarden/Ai/BP_PatrolRoute Object Reference"))
  (return (`self.PatrolRoute`)))

(fn `UserConstructionScript`)